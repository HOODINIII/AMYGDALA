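; Door Blueprint that swings its static mesh open or closed when interacted with.
; Interact checks IsOpen, sets the timeline play rate from the open or close duration, then calls OpenDoor or CloseDoor.
; One timeline, played forward or in reverse, lerps the mesh's relative yaw between closed and open positions.
; IsOpen toggles only when the timeline finishes.
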(event `Open Door`
  (bind (_direction _door_track) (`Timeline|Open Door T` :!label _label)
    (:`Update`
      (`SceneComponent.K2_SetRelativeRotation` (`self.Door SM`) (`KismetMathLibrary.MakeRotator` 0.0 0.0 (`KismetMathLibrary.Lerp` (`self.Close Position`) (`self.Open Position`) _door_track)) false false))
    (:`Finished`
      (set `self.IsOpen?` (not (`self.IsOpen?`))))))

(event `Close Door`
  (goto _label :!via `Reverse`))

(fn `Interact`
  (params (Interactor :type "Character Object Reference"))
  (returns (`Did Interact?` :type Boolean))
  (bind _open_door_t (`self.Open Door T`))
  (if (not (`self.IsOpen?`))
    (`TimelineComponent.SetPlayRate` _open_door_t (/ 1.0 (`self.Time To Open (s)`)))
    (`self.Open Door`)
    (else
      (`TimelineComponent.SetPlayRate` _open_door_t (/ 1.0 (`self.Time To Close (s)`)))
      (`self.Close Door`)))
  (return true))

(fn `UserConstructionScript`)